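; Pickup trigger actor that lets the VR pawn consume a resource while standing in its collision volume.
; Pawn overlap toggles Enabled, and the left-hand grasp input (or the A key for testing) triggers a one-time pickup.
; Only resource type 2 is handled: it calls IncreaseHunger on the pawn's StatsComponent with the resource amount, then destroys the actor.
; The ResourceManager reference is cached on BeginPlay, but its AddResources and debug-print nodes are disconnected.
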(event OnComponentBeginOverlap(CollisionComponent)
  (params (OverlappedComponent :type Primitive%20Component%20Object%20Reference) (OtherActor :type Actor%20Object%20Reference) (OtherComp :type Primitive%20Component%20Object%20Reference) (OtherBodyIndex :type Integer) (bFromSweep :type Boolean) (SweepResult :type Hit%20Result%20Structure%20%28by%20ref%29))
  ;[1 1 1] Set Trigger Collision Event
  (Utilities|Casting|CastToVRPawn OtherActor)
  (Variables|Default|Setenabled true))

(event OnComponentEndOverlap(CollisionComponent)
  (params (OverlappedComponent :type Primitive%20Component%20Object%20Reference) (OtherActor :type Actor%20Object%20Reference) (OtherComp :type Primitive%20Component%20Object%20Reference) (OtherBodyIndex :type Integer))
  ;[1 1 1] Set Trigger Collision Event
  (Utilities|Casting|CastToVRPawn OtherActor)
  (Variables|Default|Setenabled false))

(event Input|EnhancedActionEvents|EnhancedInputActionIA_Hand_Grasp_Left
  (params (ActionValue :type Float%20%28double-precision%29) (ElapsedSeconds :type Float%20%28double-precision%29) (TriggeredSeconds :type Float%20%28double-precision%29) (InputAction :type Input%20Action%20Object%20Reference :default "/Game/VRTemplate/Input/Actions/Hands/IA_Hand_Grasp_Left.IA_Hand_Grasp_Left"))
  ;[1 1 1] Create Input Event that Triggers the Resource Manager AddResource: Keyboard-> testing
  (:Triggered
    (if (Variables|Default|GetEnabled)
      (if (not (Variables|Default|GetIsPicked))
        (if (== (Variables|Default|GetResourceType) 2)
          (bind _returnvalue (Actor|GetActorOfClass "/Game/VRTemplate/Blueprints/VRPawn.VRPawn_C"))
          (bind _output_get (Variables|Components|SetStats (Actor|GetComponentbyClass _returnvalue "/Script/MyVRSurvival.StatsComponent")))
          (Class|StatsComponent|IncreaseHunger _output_get (Variables|Default|GetResourceAmount))
          (Class|StatsComponent|IncreaseHealth _output_get)
          (Variables|Default|SetIsPicked true)
          (Actor|DestroyActor))))))

(event EventBeginPlay
  ;[1 1 1] Enable Player Controller/Create Reference to VRPawn Resource Manager Actor Component
  (Input|EnableInput (Game|GetPlayerController 0))
  (bind _returnvalue (Actor|GetActorOfClass "/Game/VRTemplate/Blueprints/VRPawn.VRPawn_C"))
  (Variables|Components|SetResourceManager (Actor|GetComponentbyClass _returnvalue "/Script/MyVRSurvival.ResourceManager")))

(event Input|KeyboardEvents|A
  (params (Key :type Key%20Structure :default "None"))
  ;[1 1 1] Create Input Event that Triggers the Resource Manager AddResource: Keyboard-> testing
  (:Pressed
    (if (Variables|Default|GetEnabled)
      (if (not (Variables|Default|GetIsPicked))
        (if (== (Variables|Default|GetResourceType) 2)
          (bind _returnvalue (Actor|GetActorOfClass "/Game/VRTemplate/Blueprints/VRPawn.VRPawn_C"))
          (bind _output_get (Variables|Components|SetStats (Actor|GetComponentbyClass _returnvalue "/Script/MyVRSurvival.StatsComponent")))
          (Class|StatsComponent|IncreaseHunger _output_get (Variables|Default|GetResourceAmount))
          (Class|StatsComponent|IncreaseHealth _output_get)
          (Variables|Default|SetIsPicked true)
          (Actor|DestroyActor))))))

(fn ConstructionScript)