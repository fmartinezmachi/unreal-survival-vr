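; BP_Resource_Item is a resource item actor that removes itself from the world once collected.
; On BeginPlay it calls its parent, then binds a handler to the ItemCollected event.
; The handler destroys all descendant components of CollisionComponent, then destroys that component's owning actor.
; The construction script only calls its parent.
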(event Custom|DestroyOnCollected
  (bind _collisioncomponent (Variables|Default|GetCollisionComponent))
  ;[1 1 1] On Item Collected Destroys Components Within
  (for _array_element (Components|GetChildrenComponents _collisioncomponent true)
    (Components|DestroyComponent _array_element))
  (Actor|DestroyActor (Components|GetOwner _collisioncomponent)))

(event EventBeginPlay
  ;[1 1 1] On Item Collected Destroys Components Within
  (|CallParentFunction)
  (EventDispatchers|BindEventtoItemCollected (delegate Custom|DestroyOnCollected)))

(fn ConstructionScript
  (|CallParentFunction))