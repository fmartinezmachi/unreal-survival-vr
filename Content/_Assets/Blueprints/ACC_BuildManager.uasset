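; Actor component that handles building named items in a VR game, paid for with the player's wood, stone and metal.
; TriggerBuild skips items whose objective is already completed, then compares the VRPawn's ResourceManager totals against the item's prices.
; On success it spawns the class at the transform from the LevelManager's ACCInstantiables, deducts the cost, plays a carpenter sound and reports completion to ACCObjectiveManager.
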(event Custom|TriggerBuild
  (params (itemName :type String))
  (bind _built (CallFunction|CheckAlreadyBuilt itemName))
  (if (not _built)
    (bind _canbuild (CallFunction|CheckResources itemName))
    (if _canbuild
      (Utilities|FlowControl|Sequence
        (:then_0
          (bind _actorref (Default|GetReference() (Variables|/Game/_Assets/Blueprints/BP_LevelManager.BP_LevelManager_C|GetACC_Instantiables (Variables|Default|GetLevelManagerRef)) itemName)))
        (:then_1
          (bind _actortransform (Default|GetTransform() (Variables|/Game/_Assets/Blueprints/BP_LevelManager.BP_LevelManager_C|GetACC_Instantiables (Variables|Default|GetLevelManagerRef)) itemName)))
        (:then_2
          (Game|SpawnActorfromClass _actorref _actortransform "Undefined" 0 0)
          (bind _item (Default|GetBuildable (Variables|Default|GetLevelManagerRef) itemName))
          (CallFunction|DecreaseResources _item)
          (Audio|SpawnSoundatLocation "/Game/_Assets/Sounds/carpenter_Cue.carpenter_Cue" "0, 0, 0" "0, 0, 0" 1.0 1.0 0.0 0 0)
          (Default|OnItemCompleted (Variables|/Game/_Assets/Blueprints/BP_LevelManager.BP_LevelManager_C|GetACC_ObjectiveManager (Variables|Default|GetLevelManagerRef)) itemName))))))

(event EventBeginPlay
  (Utilities|FlowControl|Sequence
    (:then_0
      (bind _returnvalue (Actor|GetActorOfClass "/Game/_Assets/Blueprints/BP_LevelManager.BP_LevelManager_C"))
      (Variables|Default|SetLevelManagerRef _returnvalue))
    (:then_1
      (bind _returnvalue_2 (Actor|GetActorOfClass "/Game/VRTemplate/Blueprints/VRPawn.VRPawn_C"))
      (Variables|Default|SetVRPawnRef _returnvalue_2))))

(fn CheckResources
  (params (itemName :type String))
  (bind _vrpawnref (Variables|Default|GetVRPawnRef))
  (bind _resourcemanager (Variables|/Game/VRTemplate/Blueprints/VRPawn.VRPawn_C|GetResourceManager _vrpawnref))
  (bind _item (Default|GetBuildable (Variables|Default|GetLevelManagerRef) (Class|KismetStringLibrary|ToUpper itemName)))
  (bind _returnvalue (Class|ResourceManager|GetResource _resourcemanager "Wood"))
  (bind _returnvalue_2 (Class|ResourceManager|GetResource _resourcemanager "Stone"))
  (bind _returnvalue_3 (Class|ResourceManager|GetResource _resourcemanager "Metal"))
  (bind _canbuild (CallFunction|CompareResourceQuantities _returnvalue_3 _returnvalue _returnvalue_2 _item))
  (return _canbuild))

(fn CompareResourceQuantities
  (params (steel :type Integer) (wood :type Integer) (rocks :type Integer) (buildable :type BS%20Construction%20Data%20Structure))
  (bind (_prizerocks _prizesteel _prizewood) (Utilities|Struct|BreakBS_ConstructionData buildable))
  (return (Math|Boolean|ANDBoolean (>= wood _prizewood) (>= steel _prizesteel) (>= rocks _prizerocks))))

(fn CheckAlreadyBuilt
  (params (itemName :type String))
  (bind _completed (Default|ObjectiveCompleted (Variables|/Game/_Assets/Blueprints/BP_LevelManager.BP_LevelManager_C|GetACC_ObjectiveManager (Variables|Default|GetLevelManagerRef)) itemName))
  (return _completed))

(fn DecreaseResources
  (params (item :type BS%20Construction%20Data%20Structure))
  (bind (_prizerocks _prizesteel _prizewood) (Utilities|Struct|BreakBS_ConstructionData item))
  (Class|ResourceManager|RemoveResources (Variables|/Game/VRTemplate/Blueprints/VRPawn.VRPawn_C|GetResourceManager (Variables|Default|GetVRPawnRef)) "Wood" _prizewood)
  (Class|ResourceManager|RemoveResources (Variables|/Game/VRTemplate/Blueprints/VRPawn.VRPawn_C|GetResourceManager (Variables|Default|GetVRPawnRef)) "Stone" _prizerocks)
  (Class|ResourceManager|RemoveResources (Variables|/Game/VRTemplate/Blueprints/VRPawn.VRPawn_C|GetResourceManager (Variables|Default|GetVRPawnRef)) "Metal" _prizesteel))