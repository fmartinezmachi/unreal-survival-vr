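; Level manager for a VR island-escape game that handles end-of-game progression and holds the list of buildable items.
; On BeginPlay it caches the VRPawn and binds to the objective manager's all-completed event, which spawns a BP_Teleport and directs the player to the dock.
; GameCompleted shows a congratulations message in the pawn's log, then quits after a delay.
; GetBuildables and GetBuildable expose the Buildables array, the latter searching by title.
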(event Custom|CustomEvent
  (Game|SpawnActorfromClass "/Game/_Assets/Blueprints/BP_Teleport.BP_Teleport_C" (Variables|Default|GetTeleportPos) "Undefined" 0 0)
  (Default|AddMessage (Variables|Default|GetVRPawnRef) "All objectives completed, you can now go to the dock to get to the ship and leave the island."))

(event Custom|GameCompleted
  (Default|SetLogText (Variables|/Game/VRTemplate/Blueprints/VRPawn.VRPawn_C|GetUserLog (Variables|Default|GetVRPawnRef)) "Congratulations! you have managed to escape the island.")
  (Utilities|FlowControl|Delay 8.0)
  (Game|QuitGame 0 "Quit" false))

(event EventBeginPlay
  (bind _returnvalue (Actor|GetActorOfClass "/Game/VRTemplate/Blueprints/VRPawn.VRPawn_C"))
  (Variables|Default|SetVRPawnRef _returnvalue)
  (Utilities|FlowControl|Sequence
    (:then_1
      (EventDispatchers|BindEventtoAllObjectivesCompleted (Variables|Default|GetACC_ObjectiveManager) (delegate Custom|CustomEvent)))))

(fn ConstructionScript)

(fn GetBuildables
  (return (Variables|Default|GetBuildables)))

(fn GetBuildable
  (params (ItemName :type String))
  (bind _array_element (Utilities|Array|ForEachLoopwithBreak (Variables|Default|GetBuildables) :!label _label)
    (:LoopBody
      (if (Utilities|Enum|Equal(Enum) (.Title (Utilities|Struct|BreakBS_ConstructionData _array_element)) (Utilities|Text|ToText(String) ItemName))
        (Utilities|FlowControl|Sequence
          (:then_0
            (return _array_element))
          (:then_1
            (goto _label Break))
          (:then_2
            ;[1 1 1] Debuggin
            (Development|PrintString (Utilities|String|Append (Utilities|String|ToString(Text) (.Title (Utilities|Struct|BreakBS_ConstructionData _array_element))) "|" (Utilities|String|ToString(Integer) (.PrizeRocks (Utilities|Struct|BreakBS_ConstructionData _array_element))) "|" (Utilities|String|ToString(Integer) (.PrizeSteel (Utilities|Struct|BreakBS_ConstructionData _array_element))) "|" (Utilities|String|ToString(Integer) (.PrizeWood (Utilities|Struct|BreakBS_ConstructionData _array_element)))))))))))